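; BP_Bullet is a projectile actor that damages whatever it hits, other than the player who fired it.
; On BeginPlay its ammo mesh component ignores the owning player while moving.
; When its Sphere overlaps another actor, it applies a large fixed damage credited to the owner, spawns a stone impact particle at the sweep location and destroys itself.
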(event OnComponentBeginOverlap(Sphere)
  (params (OverlappedComponent :type Primitive%20Component%20Object%20Reference) (OtherActor :type Actor%20Object%20Reference) (OtherComp :type Primitive%20Component%20Object%20Reference) (OtherBodyIndex :type Integer) (bFromSweep :type Boolean) (SweepResult :type Hit%20Result%20Structure%20%28by%20ref%29))
  (if (!= OtherActor (Variables|Default|GetOwningPlayer))
    (Game|Damage|ApplyDamage OtherActor 5e+02 0 (Variables|Default|GetOwningPlayer))
    (Effects|SpawnEmitteratLocation "/Game/MilitaryWeapSilver/FX/P_Impact_Stone_Large_01.P_Impact_Stone_Large_01" (.Location (Collision|BreakHitResult SweepResult)))
    (Actor|DestroyActor)))

(event EventBeginPlay
  (Collision|IgnoreActorwhenMoving (Variables|Default|GetAssaultRifleA_Ammo) (Variables|Default|GetOwningPlayer) true))

(event Collision|EventActorBeginOverlap
  (params (OtherActor :type Actor%20Object%20Reference)))

(event EventTick
  (params (DeltaSeconds :type Float%20%28single-precision%29)))

(fn ConstructionScript)