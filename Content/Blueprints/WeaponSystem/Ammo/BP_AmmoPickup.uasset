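; BP_AmmoPickup is an ammo pickup that grants ammo to whatever overlaps its Box, through the AddAmmo message.
; One special AmmoType grants every enum type, using AmmoAmount or a default clip count looked up by the pickup's own AmmoType, not the looped one.
; Other types send AmmoAmount for that type alone.
; It plays a sound and destroys itself after the loop, or when a single-type add succeeds.
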(event OnComponentBeginOverlap(Box)
  (params (OverlappedComponent :type Primitive%20Component%20Object%20Reference) (OtherActor :type Actor%20Object%20Reference) (OtherComp :type Primitive%20Component%20Object%20Reference) (OtherBodyIndex :type Integer) (bFromSweep :type Boolean) (SweepResult :type Hit%20Result%20Structure%20%28by%20ref%29))
  (bind _ammotype (Variables|Default|GetAmmoType))
  (bind _ammoamount (Variables|Default|GetAmmoAmount))
  (bind _defaultammointheclip (Variables|DefaultAmmo|GetDefaultAmmoInTheClip))
  (bind _ammotype_2 (Variables|Default|GetAmmoType))
  (bind (_value _returnvalue) (Utilities|Map|Find _defaultammointheclip _ammotype_2))
  ;[1 1 1] Add ammo
  (if (Utilities|Enum|Equal(Enum) _ammotype "NewEnumerator3")
    (bind _enumvalue (|ForEachE_AmmoType)
      (:LoopBody
        (Class|IInteractions|AddAmmo(Message) OtherActor _enumvalue (Math|Integer|SelectInt (Math|Integer|SelectInt _value _ammoamount _returnvalue) _ammoamount (Variables|DefaultAmmo|GetDefaultAmmoCount))))
      (:then
        ;;[1 0 0] The brached is ignored here because ammo don't have limits
        (Audio|PlaySound2D "/Game/Sounds/rocketbirds/pickupammo1.pickupammo1" 1.0 1.0 0.0 0 0 :!label _label)
        (Actor|DestroyActor)))
    (else
      (bind _success (Class|IInteractions|AddAmmo(Message) OtherActor _ammotype (Variables|Default|GetAmmoAmount)))
      (if _success
        (goto _label)))))

(fn ConstructionScript)