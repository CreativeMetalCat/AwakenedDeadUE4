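; Weapon fire component that shoots BP_Bullet projectile actors when its weapon fires.
; Fire calls the parent, then spawns one bullet per BulletsPerShot, passing the weapon's damage and owner.
; Each bullet gets a random direction within a cone set by the weapon's Spread, using a random stream reseeded with a fresh random value before every spawn.
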(event EventBeginPlay
  (|CallParentFunction) ; This node is disabled and will not be called.\nDrag off pins to build functionality.
)

(event EventTick
  (params (DeltaSeconds :type Float%20%28single-precision%29))
  (|CallParentFunction DeltaSeconds) ; This node is disabled and will not be called.\nDrag off pins to build functionality.
)

(fn Fire
  (params (Location :type Vector :default "0, 0, 0") (Rotation :type Rotator :default "0, 0, 0"))
  (bind _weaponrandomstream (Variables|Default|GetWeaponRandomStream))
  (bind _weapon (Variables|Default|GetWeapon))
  (bind _weapon_2 (Variables|Default|GetWeapon))
  (bind _weaponowner (Variables|/Game/Blueprints/WeaponSystem/BP_WeaponBase.BP_WeaponBase_C|GetWeaponOwner _weapon))
  (bind _weaponinfo (Variables|/Game/Blueprints/WeaponSystem/BP_WeaponBase.BP_WeaponBase_C|GetWeaponInfo _weapon_2))
  (|CallParentFunction Location Rotation)
  (for _index (range 1 (Variables|/Game/Blueprints/WeaponSystem/BP_WeaponData.BP_WeaponData_C|GetBulletsPerShot _weaponinfo))
    (Math|Random|SetRandomStreamSeed _weaponrandomstream (Math|Random|RandomInteger 32767))
    (Game|SpawnActorfromClass "/Game/Blueprints/WeaponSystem/Projectiles/BP_Bullet.BP_Bullet_C" (Math|Transform|MakeTransform Location (Math|Rotator|FindLookatRotation Location (+ Location (* (Class|KismetMathLibrary|RandomUnitVectorinConeinRadiansfromStream (Math|Rotator|GetRotationXVector Rotation) (Math|Trig|DegreesToRadians (* (Variables|/Game/Blueprints/WeaponSystem/BP_WeaponData.BP_WeaponData_C|GetSpread _weaponinfo) 0.5)) _weaponrandomstream) 2e+02)))) "AlwaysSpawn" _weaponowner _weaponowner (Variables|/Game/Blueprints/WeaponSystem/BP_WeaponData.BP_WeaponData_C|GetDamage (Variables|/Game/Blueprints/WeaponSystem/BP_WeaponBase.BP_WeaponBase_C|GetWeaponInfo _weapon)) Location Rotation 0)))