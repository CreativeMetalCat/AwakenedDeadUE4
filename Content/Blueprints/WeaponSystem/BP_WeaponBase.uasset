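; Base weapon actor that tracks clip ammo and delegates shooting to a pluggable fire component.
; Init adds the fire component class specified in the WeaponInfo data and sets the starting clip ammo.
; Fire forwards location and rotation to that component and decrements the clip, while Reload overwrites the count.
; Getters expose weapon type, ammo type, clip state, fire readiness and automatic mode, mostly read from WeaponInfo.
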(event EventBeginPlay)

(event Collision|EventActorBeginOverlap
  (params (OtherActor :type Actor%20Object%20Reference)))

(event EventTick
  (params (DeltaSeconds :type Float%20%28single-precision%29)))

(fn ConstructionScript)

(fn Fire
  (params (Location :type Vector) (Rotation :type Rotator))
  (bind _primaryfirecomponent (Variables|Default|GetPrimaryFireComponent))
  (Utilities|IsValid _primaryfirecomponent
    (:Is%20Valid
      (Default|Fire _primaryfirecomponent Location Rotation)
      ;[1 1 1] Reduce ammo
      (Math|Integer|DecrementInt (Variables|Default|GetCurrentAmmoInTheClip)))))

(fn Init
  (params (CurrentAmmoInTheClip :type Integer))
  (bind _weaponinfo (Variables|Default|GetWeaponInfo))
  (bind _firecomponentclass (Variables|/Game/Blueprints/WeaponSystem/BP_WeaponData.BP_WeaponData_C|GetFireComponentClass _weaponinfo))
  (Utilities|IsValid _weaponinfo
    (:Is%20Valid
      (if (Utilities|IsValidClass _firecomponentclass)
        (bind _returnvalue (Game|AddComponentbyClass _firecomponentclass self))
        (Variables|Default|SetPrimaryFireComponent _returnvalue)
        (Variables|Default|SetCurrentAmmoInTheClip CurrentAmmoInTheClip)))))

(fn GetWeaponType
  (bind _weaponinfo (Variables|Default|GetWeaponInfo))
  (return (Variables|/Game/Blueprints/WeaponSystem/BP_WeaponData.BP_WeaponData_C|GetWeaponType _weaponinfo) (Utilities|IsValid _weaponinfo)))

(fn CanFire
  (return (> (Variables|Default|GetCurrentAmmoInTheClip) 0)))

(fn GetCurrentAmmointheClip
  (bind _weaponinfo (Variables|Default|GetWeaponInfo))
  (Utilities|IsValid _weaponinfo
    (:Is%20Valid
      (return (Variables|Default|GetCurrentAmmoInTheClip) (Variables|/Game/Blueprints/WeaponSystem/BP_WeaponData.BP_WeaponData_C|GetDefaultAmmoInClip _weaponinfo)))
    (:Is%20Not%20Valid
      (return -1 -1))))

(fn Reload
  (params (AmmoCount :type Integer))
  (Variables|Default|SetCurrentAmmoInTheClip AmmoCount))

(fn GetAmmoType
  (bind _weaponinfo (Variables|Default|GetWeaponInfo))
  (Utilities|IsValid _weaponinfo
    (:Is%20Valid
      (return (Variables|/Game/Blueprints/WeaponSystem/BP_WeaponData.BP_WeaponData_C|GetAmmoType _weaponinfo) true))
    (:Is%20Not%20Valid
      (return "NewEnumerator0" false))))

(fn IsAuto
  (return (Variables|/Game/Blueprints/WeaponSystem/BP_WeaponData.BP_WeaponData_C|GetAuto (Variables|Default|GetWeaponInfo))))