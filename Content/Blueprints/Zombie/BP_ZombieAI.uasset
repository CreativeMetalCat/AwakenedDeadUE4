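; AI controller for BP_Zombie that chases players or wanders to random reachable points.
; A looping timer runs either sight-perception targeting of "Player"-tagged actors or wander-only logic, chosen by UseUnitBasedAi; ChaseTarget also sets targets directly.
; Valid targets trigger move-to and chase state; otherwise wandering repeats after random cooldowns.
; Tick turns control rotation toward the target and prints its name, and the controller destroys itself when its zombie becomes invalid.
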(event Custom|UpdateAI
  (bind _aiperception (Variables|Default|GetAIPerception))
  (bind _zombie (Variables|Default|GetZombie))
  (bind _outactors (Class|AIPerceptionComponent|GetPerceivedActors _aiperception "/Script/AIModule.AISense_Sight"))
  ;[1 1 1] Ai update
  (Utilities|IsValid (Pawn|GetControlledPawn)
    (:Is%20Valid
      (if (== (Utilities|Array|FindItem _outactors (Variables|Default|GetCurrentTarget)) -1)
        ;;[1 0 0] TODO: FIND A WAY TO MAKE THIS BETTER
        (Variables|Default|SetFound true)
        (bind _array_element (Utilities|Array|ForEachLoopwithBreak _outactors :!label _label)
          (:LoopBody
            (if (!= (Utilities|Array|FindItem (Variables|/Script/Engine.Actor|GetTags _array_element) "Player") -1)
              (Variables|Default|SetCurrentTarget _array_element)
              (Variables|Default|SetFound true)
              (goto _label Break)))
          (:Completed
            ;[1 1 1] Wander around if target is null
            (if (not (Variables|Default|GetFound))
              (Variables|Default|SetCurrentTarget 0))
            (Utilities|IsValid (Variables|Default|GetCurrentTarget)
              (:Is%20Valid
                ;;[1 1 1] move to target
                (AI|Navigation|MovetoActor (stale Custom|ChaseTarget _output_get) -1.0 true true true 0 :!label _label_2)
                (Default|StartChasing (Variables|Default|GetZombie)))
              (:Is%20Not%20Valid
                (if (Variables|Default|GetWander)
                  (Utilities|IsValid _zombie
                    (:Is%20Valid
                      (Default|StopChasing _zombie)
                      (bind _returnvalue (AI|Navigation|MovetoLocation (.RandomLocation (AI|Navigation|GetRandomReachablePointinRadius (Transformation|GetActorLocation (Pawn|GetControlledPawn)) 2e+03 0 0)) -1.0 true true false true 0))
                      (switch Utilities|FlowControl|Switch|SwitchonEPathFollowingRequestResult _returnvalue
                        (:RequestSuccessful
                          (Utilities|Time|SetTimerbyEvent (delegate Custom|ResetRandomMovementCooldown) (Math|Random|RandomFloatinRange 3.0 1e+01))
                          (Variables|Default|SetWander false))))
                    (:Is%20Not%20Valid
                      (Actor|DestroyActor))))))))
        (else
          (goto _label_2))))
    (:Is%20Not%20Valid
      (Actor|DestroyActor))))

(event Custom|ResetRandomMovementCooldown
  (Variables|Default|SetWander true))

(event Custom|WanderAround
  (bind _zombie (Variables|Default|GetZombie))
  ;[1 1 1] Wander around if target is null
  (Utilities|IsValid (Variables|Default|GetCurrentTarget)
    (:Is%20Valid
      ;[1 1 1] Ai update
      ;;[1 1 1] move to target
      (AI|Navigation|MovetoActor (stale Custom|ChaseTarget _output_get) -1.0 true true true 0)
      (Default|StartChasing (Variables|Default|GetZombie)))
    (:Is%20Not%20Valid
      (if (Variables|Default|GetWander)
        (Utilities|IsValid _zombie
          (:Is%20Valid
            (Default|StopChasing _zombie)
            (bind _returnvalue (AI|Navigation|MovetoLocation (.RandomLocation (AI|Navigation|GetRandomReachablePointinRadius (Transformation|GetActorLocation (Pawn|GetControlledPawn)) 2e+03 0 0)) -1.0 true true false true 0))
            (switch Utilities|FlowControl|Switch|SwitchonEPathFollowingRequestResult _returnvalue
              (:RequestSuccessful
                (Utilities|Time|SetTimerbyEvent (delegate Custom|ResetRandomMovementCooldown) (Math|Random|RandomFloatinRange 3.0 1e+01))
                (Variables|Default|SetWander false))))
          (:Is%20Not%20Valid
            (Actor|DestroyActor)))))))

(event Custom|ChaseTarget
  (params (target :type Actor%20Object%20Reference))
  ;[1 1 1] Ai update
  ;;[1 1 1] move to target
  (bind _output_get (Variables|Default|SetCurrentTarget target))
  (AI|Navigation|MovetoActor _output_get -1.0 true true true 0)
  (Default|StartChasing (Variables|Default|GetZombie)))

(event Custom|StopChasing
  (bind _zombie (Variables|Default|GetZombie))
  ;[1 1 1] Stop chasing
  (Utilities|IsValid _zombie
    (:Is%20Valid
      (Default|StopChasing _zombie))
    (:Is%20Not%20Valid
      (Actor|DestroyActor))))

(event EventBeginPlay
  ;[1 1 1] begin play
  (Utilities|Time|SetTimerbyEvent (select (Variables|Default|GetUseUnitBasedAi) (delegate Custom|UpdateAI) (delegate Custom|WanderAround)) 0.5 true)
  ;[1 1 1] cache zombie pawn
  (bind _asbp_zombie (Utilities|Casting|CastToBP_Zombie (Pawn|GetControlledPawn) :!label _label)
    (:then
      (Variables|Default|SetZombie _asbp_zombie))
    (:CastFailed
      _))
  (Utilities|IsValid (Variables|Default|GetZombie)
    (:Is%20Not%20Valid
      (Utilities|FlowControl|Delay 0.1)
      (goto _label))))

(event EventTick
  (params (DeltaSeconds :type Float%20%28single-precision%29))
  (bind _returnvalue (Pawn|GetControlledPawn))
  (bind _currenttarget (Variables|Default|GetCurrentTarget))
  ;[1 1 1] Tick
  (Utilities|IsValid _currenttarget
    (:Is%20Valid
      (Utilities|IsValid _returnvalue
        (:Is%20Valid
          (Pawn|SetControlRotation (Math|Rotator|FindLookatRotation (Transformation|GetActorLocation _returnvalue) (Transformation|GetActorLocation _currenttarget)))
          (Development|PrintString (Utilities|GetDisplayName _currenttarget) true true "(R=0.000000,G=0.660000,B=1.000000,A=1.000000)" DeltaSeconds))))))

(fn ConstructionScript)