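; Zombie enemy character that chases and melees BP_Player, takes point damage and ragdolls on death.
; A half-second Tick checks AttackCollision for players, slowing movement and picking a random AttackType; Attack applies damage to the first overlapping player.
; Point damage spawns blood effects, then either calls Die or plays a hit montage via server-to-multicast events, with notifies adjusting speed.
; StartChasing and StopChasing toggle chase state and walk speed.
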(event Custom|PlayMontageMultiCast
  (params (MontageToPlay :type Anim%20Montage%20Object%20Reference) (Action :type E_MontageActionType%20Enum :default "NewEnumerator0"))
  (bind _charactermovement (Variables|Character|GetCharacterMovement))
  ;[1 1 1] Replication of the montages
  (Animation|Montage|PlayMontage (Variables|Character|GetMesh) MontageToPlay
    (:OnNotifyBegin
      ;[1 1 1] On Montage Notify Begin and End
      (Variables|/Script/Engine.CharacterMovementComponent|SetMaxWalkSpeed _charactermovement (* (Variables|/Script/Engine.CharacterMovementComponent|GetMaxWalkSpeed _charactermovement) 0.75)))
    (:OnNotifyEnd
      (Variables|/Script/Engine.CharacterMovementComponent|SetMaxWalkSpeed _charactermovement (Variables|Default|GetDefaultMovementSpeed)))))

(event Custom|PlayMontageOnServer
  (params (MontageToPlay :type Anim%20Montage%20Object%20Reference) (Action :type E_MontageActionType%20Enum :default "NewEnumerator0"))
  ;[1 1 1] Replication of the montages
  (CallFunction|PlayMontageMultiCast MontageToPlay Action))

(event EventTick
  (params (DeltaSeconds :type Float%20%28single-precision%29))
  (bind _attackcollision (Variables|Default|GetAttackCollision))
  (bind _overlappingactors (Collision|GetOverlappingActors _attackcollision "/Game/Blueprints/Player/BP_Player.BP_Player_C" :!class /Script/Engine.PrimitiveComponent))
  (bind _returnvalue (Utilities|Array|Length _overlappingactors))
  (bind _returnvalue_2 (> _returnvalue 0))
  ;[1 1 1] TICK
  (if (not (Variables|Default|GetDead))
    (if (not (Variables|Default|GetAttacking))
      (if _returnvalue_2
        (Variables|Default|SetAttacking true)
        (Variables|Default|SetAttackType (Math|Random|RandomIntegerinRange 1 4))
        (Variables|/Script/Engine.CharacterMovementComponent|SetMaxWalkSpeed (Variables|Character|GetCharacterMovement) (/ (Variables|Default|GetDefaultMovementSpeed) 4.0))
        (else
          (Variables|Default|SetAttacking false :!label _label)
          (Variables|/Script/Engine.CharacterMovementComponent|SetMaxWalkSpeed (Variables|Character|GetCharacterMovement) (Variables|Default|GetDefaultMovementSpeed))))
      (elif (not _returnvalue_2)
        (goto _label)))))

(event Game|Damage|EventPointDamage
  (params (Damage :type Float%20%28single-precision%29) (DamageType :type Damage%20Type%20Object%20Reference) (HitLocation :type Vector :default "0, 0, 0") (HitNormal :type Vector :default "0, 0, 0") (HitComponent :type Primitive%20Component%20Object%20Reference) (BoneName :type Name :default "None") (ShotFromDirection :type Vector :default "0, 0, 0") (InstigatedBy :type Controller%20Object%20Reference) (DamageCauser :type Actor%20Object%20Reference) (HitInfo :type Hit%20Result%20Structure%20%28by%20ref%29))
  (bind (_bblockinghit _binitialoverlap _time _distance _location _impactpoint _normal _impactnormal _physmat _hitactor _hitcomponent _hitbonename _hititem _faceindex _tracestart _traceend) (Collision|BreakHitResult HitInfo))
  (bind _returnvalue (Math|Rotator|FindLookatRotation _tracestart _traceend))
  ;[0.03212 0 1] Receive damage
  (bind _output_get (Variables|Default|SetHealth (- (Variables|Default|GetHealth) Damage)))
  (Niagara|SpawnSystematLocation "/Game/Particles/Blood/NS_Blood.NS_Blood" _location _returnvalue "10.000000,10.000000,10.000000")
  (Effects|SpawnEmitteratLocation "/Game/MilitaryWeapSilver/FX/P_Impact_Flesh.P_Impact_Flesh" _location _returnvalue)
  (if (<= _output_get 0.0)
    (CallFunction|Die)
    (else
      ;;[0 1 0.5375] Play hit anim
      (CallFunction|PlayMontageonServer "/Game/MonsterZombie/Animations/Anim_Zombie_hit1_Montage.Anim_Zombie_hit1_Montage" "NewEnumerator0")
      (Audio|Components|Audio|Play (Variables|Default|GetHitSound) 0.0))))

(fn ConstructionScript
  (Variables|Default|SetDefaultMovementSpeed (Variables|/Script/Engine.CharacterMovementComponent|GetMaxWalkSpeed (Variables|Character|GetCharacterMovement))))

(fn Die
  (bind _returnvalue (Pawn|GetController))
  (bind _mesh (Variables|Character|GetMesh))
  (Collision|SetCollisionEnabled _mesh "PhysicsOnly")
  (Physics|SetSimulatePhysics _mesh true)
  (Utilities|IsValid _returnvalue
    (:Is%20Valid
      (Pawn|UnPossess _returnvalue))
    (:Is%20Not%20Valid
      _))
  (Collision|SetCollisionEnabled (Variables|Collision|GetCapsuleComponent) "NoCollision")
  (Audio|Components|Audio|Play (Variables|Default|GetHitSound) 0.0)
  (Variables|Default|SetDead true))

(fn Attack
  (if (not (Variables|Default|GetDead))
    (Game|Damage|ApplyDamage (Utilities|Array|Get(acopy) (Collision|GetOverlappingActors (Variables|Default|GetAttackCollision) "/Game/Blueprints/Player/BP_Player.BP_Player_C" :!class /Script/Engine.PrimitiveComponent)) (Variables|Damage|GetDamage) 0 self)))

(fn StartChasing
  (Variables|Default|SetChasing true)
  (Variables|/Script/Engine.CharacterMovementComponent|SetMaxWalkSpeed (Variables|Character|GetCharacterMovement) (Variables|Default|GetDefaultMovementSpeed)))

(fn StopChasing
  (Variables|Default|SetChasing false)
  (Variables|/Script/Engine.CharacterMovementComponent|SetMaxWalkSpeed (Variables|Character|GetCharacterMovement) (/ (Variables|Default|GetDefaultMovementSpeed) 3.0)))