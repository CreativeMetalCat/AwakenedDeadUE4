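; BP_AiManager is a zombie manager that directs a group of AI pawns to chase actors entering its sphere trigger.
; An overlapping actor with EnemyTag becomes CurrentTarget, and each pawn's BP_ZombieAI controller is told to chase it.
; Any actor leaving the sphere, not just the current target, clears the target and stops the chase.
; That end-overlap loop also removes invalid entries from the AI array while iterating it.
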(event OnComponentBeginOverlap(Sphere)
  (params (OverlappedComponent :type Primitive%20Component%20Object%20Reference) (OtherActor :type Actor%20Object%20Reference) (OtherComp :type Primitive%20Component%20Object%20Reference) (OtherBodyIndex :type Integer) (bFromSweep :type Boolean) (SweepResult :type Hit%20Result%20Structure%20%28by%20ref%29))
  ;[1 1 1] Update target
  (if (!= (Utilities|Array|FindItem (Variables|/Script/Engine.Actor|GetTags OtherActor) (Variables|Default|GetEnemyTag)) -1)
    (Variables|Default|SetCurrentTarget OtherActor)
    (for _array_element (Variables|Default|GetAI)
      (bind _asbp_zombie_ai (Utilities|Casting|CastToBP_ZombieAI (Pawn|GetController _array_element)))
      (Default|ChaseTarget _asbp_zombie_ai (Variables|Default|GetCurrentTarget)))))

(event OnComponentEndOverlap(Sphere)
  (params (OverlappedComponent :type Primitive%20Component%20Object%20Reference) (OtherActor :type Actor%20Object%20Reference) (OtherComp :type Primitive%20Component%20Object%20Reference) (OtherBodyIndex :type Integer))
  (bind _ai (Variables|Default|GetAI))
  ;[1 1 1] Stop chasing if target left
  (Variables|Default|SetCurrentTarget 0)
  (for _array_element _ai
    (Utilities|IsValid _array_element
      (:Is%20Valid
        (bind _asbp_zombie_ai (Utilities|Casting|CastToBP_ZombieAI (Pawn|GetController _array_element)))
        (Default|StopChasing _asbp_zombie_ai))
      (:Is%20Not%20Valid
        (Utilities|Array|RemoveItem _ai _array_element)))))

(event EventBeginPlay)

(event Collision|EventActorBeginOverlap
  (params (OtherActor :type Actor%20Object%20Reference)))

(event EventTick
  (params (DeltaSeconds :type Float%20%28single-precision%29)))

(fn ConstructionScript)