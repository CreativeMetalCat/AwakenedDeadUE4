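; BP_Spawner spawns a crowd of zombies from AllowedTypes at random navigable points within a Radius shown by its Sphere component.
; On BeginPlay it finds the level's BP_AiManager if unset, printing a red warning when none exists.
; Spawn, not called within this Blueprint, creates MaxAmount plus a random variation, registering each zombie with the manager.
; Each zombie's OnDeath is bound to decrement CurrentAmount, which Spawn never increments.
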(event Custom|BindZombieDeathEvent
  (params (Zombie :type BP%20Zombie%20Object%20Reference))
  ;[1 1 1] Bind death event
  (EventDispatchers|BindEventtoOnDeath Zombie (delegate Custom|OnZombieDied)))

(event Custom|OnZombieDied
  ;[1 1 1] Begin play
  (Math|Integer|DecrementInt (Variables|Default|GetCurrentAmount)))

(event EventBeginPlay
  ;[1 1 1] Begin play
  (Utilities|IsValid (Variables|AiManager|GetAiManager)
    (:Is%20Not%20Valid
      (bind _outactors (Actor|GetAllActorsOfClass "/Game/Blueprints/Zombie/BP_AiManager.BP_AiManager_C"))
      (Variables|AiManager|SetAiManager (Utilities|Array|Get(acopy) _outactors))
      (Utilities|IsValid (Variables|AiManager|GetAiManager)
        (:Is%20Not%20Valid
          (Development|PrintString "No AiManager is present on the map. Please add one for crowd ai to work!" true true "(R=1.000000,G=0.000000,B=0.000000,A=1.000000)"))))))

(event Collision|EventActorBeginOverlap
  (params (OtherActor :type Actor%20Object%20Reference)))

(event EventTick
  (params (DeltaSeconds :type Float%20%28single-precision%29)))

(fn ConstructionScript
  (Components|Sphere|SetSphereRadius (Variables|Default|GetSphere) (Variables|Default|GetRadius) false))

(fn Spawn
  (bind _allowedtypes (Variables|Default|GetAllowedTypes))
  (bind _aimanager (Variables|AiManager|GetAiManager))
  (bind _outitem (Utilities|Array|Random _allowedtypes))
  (if (> (Variables|Amount|GetMaxAmount) 0)
    (for _index (range 0 (+ (Variables|Amount|GetMaxAmount) (Math|Random|RandomIntegerinRange 0 (Variables|Amount|GetMaxVariation))))
      ;[1 1 1] Spawn and bind events
      (bind _returnvalue (Game|SpawnActorfromClass _outitem (Math|Transform|MakeTransform (.RandomLocation (Class|NavigationSystemV1|GetRandomPointinNavigableRadius (Transformation|GetActorLocation) (Variables|Default|GetRadius) 0 0))) "AdjustIfPossibleButAlwaysSpawn" 0 (.Health (Utilities|GetClassDefaults _outitem)) 0 0))
      (CallFunction|BindZombieDeathEvent _returnvalue)
      ;[1 1 1] Add zombie to manager
      (Utilities|Array|Add (Variables|/Game/Blueprints/Zombie/BP_AiManager.BP_AiManager_C|GetAI _aimanager) _returnvalue)
      (Development|PrintString (Utilities|GetDisplayName _aimanager)))))